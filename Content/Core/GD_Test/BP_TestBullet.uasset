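; BP_TestBullet is a test projectile actor that deals damage to whatever its sphere overlaps, then destroys itself.
; A settype event switches the sphere between fire and water shield materials, changing only its look.
; BeginPlay and a second custom event share one path that stores the ProjectileMovement max speed in IABulletSpeed.
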(event OnComponentBeginOverlap(Sphere)
  (params (OverlappedComponent :type Primitive%20Component%20Object%20Reference) (OtherActor :type Actor%20Object%20Reference) (OtherComp :type Primitive%20Component%20Object%20Reference) (OtherBodyIndex :type Integer) (bFromSweep :type Boolean) (SweepResult :type Hit%20Result%20Structure%20%28by%20ref%29))
  (Game|Damage|ApplyDamage OtherActor 1.0 0 self)
  (Actor|DestroyActor))

(event Custom|reste%20begin$
  (Utilities|FlowControl|Sequence
    (:then_1
      (Variables|Parameters|SetIA_Bullet_Speed (Class|MovementComponent|GetMaxSpeed (Variables|Default|GetProjectileMovement))))))

(event Custom|set%20type
  (params (Fire? :type Boolean))
  (bind _sphere (Variables|Default|GetSphere))
  (if Fire?
    (Rendering|Material|SetMaterial _sphere 0 "/Game/Core/Material/Inst/M_Shield_Fire_Inst.M_Shield_Fire_Inst")
    (else
      (Rendering|Material|SetMaterial _sphere 0 "/Game/Core/Material/Inst/M_Shield_Water_Inst.M_Shield_Water_Inst"))))

(event EventBeginPlay
  (Utilities|FlowControl|Sequence
    (:then_1
      (Variables|Parameters|SetIA_Bullet_Speed (Class|MovementComponent|GetMaxSpeed (Variables|Default|GetProjectileMovement))))))

(fn ConstructionScript)