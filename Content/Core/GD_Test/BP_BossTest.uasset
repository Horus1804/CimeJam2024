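; Test boss that takes over when the camera enters its trigger box, stopping camera tick, flagging the player and removing the AI spawner.
; A self-repeating Shoot event randomly alternates sweep and shotgun patterns across three cannons, spawning bullets with randomized type, optional stagger and jittered sweep angles.
; Each hit decrements boss life; at zero it shows the end-level widget and destroys itself.
; While activated, Tick drifts it along X.
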(event OnComponentBeginOverlap(Box)
  (params (OverlappedComponent :type Primitive%20Component%20Object%20Reference) (OtherActor :type Actor%20Object%20Reference) (OtherComp :type Primitive%20Component%20Object%20Reference) (OtherBodyIndex :type Integer) (bFromSweep :type Boolean) (SweepResult :type Hit%20Result%20Structure%20%28by%20ref%29))
  (Utilities|Casting|CastToBP_Camera OtherActor)
  (Utilities|FlowControl|DoOnce false
    (:Completed
      (CallFunction|Shoot)
      (Collision|SetCollisionEnabled (Variables|Default|GetBox) "NoCollision")
      (Actor|Tick|SetActorTickEnabled (Variables|Default|GetCamera_Ref))
      (Variables|/Game/Core/Bleuprint/Player/BP_Player.BP_Player_C|SetKill_Tick_For_Boss (Variables|/Game/Core/Bleuprint/Camera/BP_Camera.BP_Camera_C|GetRefPlayer (Variables|Default|GetCamera_Ref)) true)
      (bind _returnvalue (Actor|GetActorOfClass "/Game/Core/Bleuprint/AI-Ennemy/BP_SpawnAI.BP_SpawnAI_C"))
      (Utilities|IsValid _returnvalue
        (:Is%20Valid
          (Actor|DestroyActor _returnvalue))))))

(event Custom|BalayageHaut
  (params (Fire? :type Boolean) (Delay :type Boolean) (Alternate? :type Boolean) (AimArray :type Array%20of%20Floats%20%28double-precision%29))
  (Variables|Default|SetCompteurHaut 0)
  (if (!= (Utilities|Array|Length AimArray) (Variables|Default|GetCompteurHaut)) :!label _label
    (bind _returnvalue (Game|SpawnActorfromClass "/Game/Core/GD_Test/BP_TestBullet.BP_TestBullet_C" (Math|Transform|MakeTransform (Transformation|GetWorldLocation (Variables|Default|GetUpperCannon)) (Math|Rotator|MakeRotator 0.0 (+ (Utilities|Array|Get(acopy) AimArray (Variables|Default|GetCompteurHaut)) (* (Math|Random|RandomFloat) 5.0)) 0.0) "1.000000,1.000000,1.000000") "AlwaysSpawn" "MultiplyWithRoot" 0 0))
    (if Alternate?
      (Default|SetType _returnvalue (Math|Conversions|ToBoolean(Integer) (Math|Integer|%(Integer) (Variables|Default|GetCompteurHaut) 2)))
      (else
        (Default|SetType _returnvalue Fire?)))
    (Variables|Default|SetCompteurHaut (+ (Variables|Default|GetCompteurHaut) 1))
    (if Delay
      (Utilities|FlowControl|Delay 0.05)
      (goto _label)
      (else
        (goto _label)))))

(event Custom|ShotgunMilieu
  (params (Fire? :type Boolean))
  (for _array_element (Variables|Default|GetShotgunArray)
    (bind _returnvalue (Game|SpawnActorfromClass "/Game/Core/GD_Test/BP_TestBullet.BP_TestBullet_C" (Math|Transform|MakeTransform (Transformation|GetWorldLocation (Variables|Default|GetMiddleCannon)) (Math|Rotator|MakeRotator 0.0 (+ _array_element 1.8e+02) 0.0) "1.000000,1.000000,1.000000") "Undefined" "MultiplyWithRoot" 0 0))
    (Default|SetType _returnvalue Fire?)))

(event Custom|Shoot
  (bind _returnvalue (Math|Random|RandomBool))
  (bind _returnvalue_2 (Math|Random|RandomInteger 2))
  (bind _returnvalue_3 (Math|Random|RandomBool))
  (bind _returnvalue_4 (Math|Random|RandomBool))
  (bind _outtoinarray (Variables|Default|GetOutToInArray))
  (bind _intooutarray (Variables|Default|GetInToOutArray))
  (bind _returnvalue_5 (Utilities|Select :Index _returnvalue_2 :Option%200 _outtoinarray :Option%201 _intooutarray))
  (if (Math|Random|RandomBool)
    (Variables|Default|SetDelay? _returnvalue_3)
    (Variables|Default|SetUpperFire? _returnvalue_3)
    (Variables|Default|SetLowerFire? _returnvalue_3)
    (Variables|Default|SetAlternate _returnvalue_3)
    (CallFunction|BalayageHaut (Variables|Default|GetUpperFire?) (Variables|Default|GetDelay?) (Variables|Default|GetAlternate) _returnvalue_5)
    (CallFunction|BalayageBas (Variables|Default|GetLowerFire?) (Variables|Default|GetDelay?) (Variables|Default|GetAlternate) _returnvalue_5)
    (CallFunction|ShotgunMilieu _returnvalue_3)
    (if (Variables|Default|GetDelay?)
      (Utilities|FlowControl|Delay 2.0)
      (else
        (Utilities|FlowControl|Delay 1.0)))
    (CallFunction|Shoot)
    (else
      (bind _output_get (Variables|Default|SetDelay? _returnvalue))
      (bind _output_get_2 (Variables|Default|SetUpperFire? _returnvalue))
      (Variables|Default|SetLowerFire? _returnvalue)
      (bind _output_get_3 (Variables|Default|SetAlternate _returnvalue))
      (CallFunction|BalayageMilieu _output_get_2 _output_get _output_get_3)
      (CallFunction|ShotgunBas _returnvalue_4)
      (CallFunction|ShotgunHaut _returnvalue_4)
      (if _output_get
        (Utilities|FlowControl|Delay 2.0)
        (else
          (Utilities|FlowControl|Delay 1.0)))
      (CallFunction|Shoot))))

(event Custom|BalayageBas
  (params (Fire? :type Boolean) (Delay? :type Boolean) (Alternate :type Boolean) (AimArray :type Array%20of%20Floats%20%28double-precision%29))
  (bind _returnvalue (Utilities|Array|Length AimArray))
  (Variables|Default|SetCompteurBas 0)
  (if (!= _returnvalue (Variables|Default|GetCompteurBas)) :!label _label
    (bind _returnvalue_2 (Game|SpawnActorfromClass "/Game/Core/GD_Test/BP_TestBullet.BP_TestBullet_C" (Math|Transform|MakeTransform (Transformation|GetWorldLocation (Variables|Default|GetLowerCannon)) (Math|Rotator|MakeRotator 0.0 (+ (Utilities|Array|Get(acopy) AimArray (+ (- _returnvalue (Variables|Default|GetCompteurBas)) -1)) (* (Math|Random|RandomFloat) 5.0)) 0.0) "1.000000,1.000000,1.000000") "AlwaysSpawn" "MultiplyWithRoot" 0 0))
    (if Alternate
      (Default|SetType _returnvalue_2 (Math|Conversions|ToBoolean(Integer) (Math|Integer|%(Integer) (Variables|Default|GetCompteurBas) 2)))
      (else
        (Default|SetType _returnvalue_2 Fire?)))
    (Variables|Default|SetCompteurBas (+ (Variables|Default|GetCompteurBas) 1))
    (if Delay?
      (Utilities|FlowControl|Delay 0.05)
      (goto _label)
      (else
        (goto _label)))))

(event Custom|BalayageMilieu
  (params (Fire :type Boolean) (Delay :type Boolean) (Alternate :type Boolean))
  (if Delay
    (Variables|Default|SetCompteurMilieu 0)
    (if (!= (Utilities|Array|Length (Variables|Default|GetOutToInArray)) (Variables|Default|GetCompteurMilieu)) :!label _label
      (bind _returnvalue (Game|SpawnActorfromClass "/Game/Core/GD_Test/BP_TestBullet.BP_TestBullet_C" (Math|Transform|MakeTransform (Transformation|GetWorldLocation (Variables|Default|GetMiddleCannon)) (Math|Rotator|MakeRotator 0.0 (+ (Utilities|Array|Get(acopy) (Variables|Default|GetOutToInArray) (Variables|Default|GetCompteurMilieu)) (* (Math|Random|RandomFloat) 5.0)) 0.0) "1.000000,1.000000,1.000000") "AlwaysSpawn" "MultiplyWithRoot" 0 0))
      (if Alternate
        (Default|SetType _returnvalue (Math|Conversions|ToBoolean(Integer) (Math|Integer|%(Integer) (Variables|Default|GetCompteurMilieu) 2)))
        (else
          (Default|SetType _returnvalue (Variables|Default|GetLowerFire?))))
      (bind _returnvalue_2 (Game|SpawnActorfromClass "/Game/Core/GD_Test/BP_TestBullet.BP_TestBullet_C" (Math|Transform|MakeTransform (Transformation|GetWorldLocation (Variables|Default|GetMiddleCannon)) (Math|Rotator|MakeRotator 0.0 (+ (Utilities|Array|Get(acopy) (Variables|Default|GetInToOutArray) (Variables|Default|GetCompteurMilieu)) (* (Math|Random|RandomFloat) 5.0)) 0.0) "1.000000,1.000000,1.000000") "AlwaysSpawn" "MultiplyWithRoot" 0 0))
      (if true
        (Default|SetType _returnvalue_2 (Math|Conversions|ToBoolean(Integer) (Math|Integer|%(Integer) (Variables|Default|GetCompteurMilieu) 2)))
        (else
          (Default|SetType _returnvalue_2 (Variables|Default|GetUpperFire?))))
      (Variables|Default|SetCompteurMilieu (+ (Variables|Default|GetCompteurMilieu) 1))
      (Utilities|FlowControl|Delay 0.05)
      (goto _label))
    (else
      (Variables|Default|SetCompteurMilieu 0)
      (if (!= (Utilities|Array|Length (Variables|Default|GetOutToInArray)) (Variables|Default|GetCompteurMilieu)) :!label _label_2
        (bind _returnvalue_3 (Game|SpawnActorfromClass "/Game/Core/GD_Test/BP_TestBullet.BP_TestBullet_C" (Math|Transform|MakeTransform (Transformation|GetWorldLocation (Variables|Default|GetMiddleCannon)) (Math|Rotator|MakeRotator 0.0 (+ (Utilities|Array|Get(acopy) (Variables|Default|GetOutToInArray) (Variables|Default|GetCompteurMilieu)) (* (Math|Random|RandomFloat) 5.0)) 0.0) "1.000000,1.000000,1.000000") "AlwaysSpawn" "MultiplyWithRoot" 0 0))
        (if Alternate
          (Default|SetType _returnvalue_3 (Math|Conversions|ToBoolean(Integer) (Math|Integer|%(Integer) (Variables|Default|GetCompteurMilieu) 2)))
          (else
            (Default|SetType _returnvalue_3 Fire)))
        (Variables|Default|SetCompteurMilieu (+ (Variables|Default|GetCompteurMilieu) 1))
        (goto _label_2)))))

(event Custom|ShotgunHaut
  (params (Fire? :type Boolean))
  (for _array_element (Variables|Default|GetShotgunArray)
    (bind _returnvalue (Game|SpawnActorfromClass "/Game/Core/GD_Test/BP_TestBullet.BP_TestBullet_C" (Math|Transform|MakeTransform (Transformation|GetWorldLocation (Variables|Default|GetUpperCannon)) (Math|Rotator|MakeRotator 0.0 (+ _array_element 175.0) 0.0) "1.000000,1.000000,1.000000") "Undefined" "MultiplyWithRoot" 0 0))
    (Default|SetType _returnvalue Fire?)))

(event Custom|ShotgunBas
  (params (Fire? :type Boolean))
  (for _array_element (Variables|Default|GetShotgunArray)
    (bind _returnvalue (Game|SpawnActorfromClass "/Game/Core/GD_Test/BP_TestBullet.BP_TestBullet_C" (Math|Transform|MakeTransform (Transformation|GetWorldLocation (Variables|Default|GetLowerCannon)) (Math|Rotator|MakeRotator 0.0 (+ _array_element 185.0) 0.0) "1.000000,1.000000,1.000000") "Undefined" "MultiplyWithRoot" 0 0))
    (Default|SetType _returnvalue Fire?)))

(event Game|Damage|EventAnyDamage
  (params (Damage :type Float%20%28single-precision%29) (DamageType :type Damage%20Type%20Object%20Reference) (InstigatedBy :type Controller%20Object%20Reference) (DamageCauser :type Actor%20Object%20Reference))
  (bind _result (Math|Integer|DecrementInt (Variables|Default|GetBoss_Life))
    (:%20%20
      (if (<= _result 0)
        (Utilities|FlowControl|DoOnce false
          (:Completed
            (bind _returnvalue (UserInterface|CreateWidget "/Game/Core/Bleuprint/UI/WBP_EndLevel.WBP_EndLevel_C"))
            (Variables|/Game/Core/Bleuprint/UI/WBP_EndLevel.WBP_EndLevel_C|SetPlayerRef _returnvalue (Variables|/Game/Core/Bleuprint/Camera/BP_Camera.BP_Camera_C|GetRefPlayer (Variables|Default|GetCamera_Ref)))
            (UserInterface|Viewport|AddtoViewport _returnvalue 0)
            (Actor|DestroyActor)))))))

(event EventTick
  (params (DeltaSeconds :type Float%20%28single-precision%29))
  (if (Variables|Default|GetActivated)
    (Transformation|SetActorLocation (+ (Transformation|GetActorLocation) "1.000000,0.000000,0.000000") false false)))

(fn ConstructionScript)