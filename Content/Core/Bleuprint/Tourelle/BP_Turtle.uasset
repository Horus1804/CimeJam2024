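; BP_Turtle is a turret actor that rotates its cannon bone to follow the player.
; On BeginPlay it plays a one-shot animation, then after a short delay hides the skeletal mesh, shows a poseable mesh and enables Tick.
; Each Tick finds BP_Player and drives "rot_canon" in component space from the player-to-turret look-at rotation with remapped axes, printing that rotation as debug output.
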(event EventBeginPlay
  (Components|Animation|PlayAnimation (Variables|Default|GetSkeletalMesh) "/Game/Core/Game_art/Zeplin_et_ennemie/tourelle_animation/tourelle_Anim.tourelle_Anim" false)
  (Utilities|FlowControl|Delay 1.2)
  (Rendering|SetVisibility (Variables|Default|GetSkeletalMesh) false false)
  (Rendering|SetVisibility (Variables|Default|GetPoseableMesh) true false)
  (Actor|Tick|SetActorTickEnabled true))

(event Collision|EventActorBeginOverlap
  (params (OtherActor :type Actor%20Object%20Reference)))

(event EventTick
  (params (DeltaSeconds :type Float%20%28single-precision%29))
  (bind _returnvalue (Actor|GetActorOfClass "/Game/Core/Bleuprint/Player/BP_Player.BP_Player_C"))
  (Development|PrintString (Utilities|String|ToString(Rotator) (Math|Rotator|FindLookatRotation (Transformation|GetActorLocation _returnvalue) (Transformation|GetActorLocation))))
  (Components|PoseableMesh|SetBoneRotationbyName (Variables|Default|GetPoseableMesh) "rot_canon" (Math|Rotator|MakeRotator (.Pitch (Math|Rotator|BreakRotator (Math|Rotator|FindLookatRotation (Transformation|GetActorLocation _returnvalue) (Transformation|GetActorLocation)))) (.Yaw (Math|Rotator|BreakRotator (Math|Rotator|FindLookatRotation (Transformation|GetActorLocation _returnvalue) (Transformation|GetActorLocation)))) (.Roll (Math|Rotator|BreakRotator (Math|Rotator|FindLookatRotation (Transformation|GetActorLocation _returnvalue) (Transformation|GetActorLocation))))) "ComponentSpace"))

(fn ConstructionScript)