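; Enemy AI projectile Blueprint that damages whatever it overlaps, with visuals matching the firing enemy's element.
; A settype event takes an enemy reference and swaps the particle template to Fire or Water based on its element enum.
; On BeginPlay it caches the projectile movement's max speed.
; Sphere overlap applies fixed damage to the other actor, then destroys the bullet.
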(event OnComponentBeginOverlap(Sphere1)
  (params (OverlappedComponent :type Primitive%20Component%20Object%20Reference) (OtherActor :type Actor%20Object%20Reference) (OtherComp :type Primitive%20Component%20Object%20Reference) (OtherBodyIndex :type Integer) (bFromSweep :type Boolean) (SweepResult :type Hit%20Result%20Structure%20%28by%20ref%29))
  (Game|Damage|ApplyDamage OtherActor 1.0 0 self)
  (Actor|DestroyActor))

(event Custom|reste%20begin$
  (Utilities|FlowControl|Sequence
    (:then_1
      (Variables|Parameters|SetIA_Bullet_Speed (Class|MovementComponent|GetMaxSpeed (Variables|Default|GetProjectileMovement))))))

(event Custom|set%20type
  (params (IA_Ennemy_Ref :type BP%20AI%20Ennemy%20Object%20Reference))
  (Utilities|IsValid IA_Ennemy_Ref
    (:Is%20Valid
      (bind _output_get (Variables|BP_Ref|SetIA_Ennemy_Ref IA_Ennemy_Ref))
      (switch Utilities|FlowControl|Switch|SwitchonE_IA_Ennemy_Elements (Variables|/Game/Core/Bleuprint/AI-Ennemy/BP_AI_Ennemy.BP_AI_Ennemy_C|GetE_AI_Elements _output_get)
        (:NewEnumerator0
          (Effects|Components|ParticleSystem|SetTemplate (Variables|Default|GetParticleSystem) "/Game/Core/VFX/Luos8Elements/Particles/Fire/fire_particules_test.fire_particules_test"))
        (:NewEnumerator1
          (Effects|Components|ParticleSystem|SetTemplate (Variables|Default|GetParticleSystem) "/Game/Core/VFX/Luos8Elements/Particles/Aqua/water_particules_test.water_particules_test"))))))

(event EventBeginPlay
  (Utilities|FlowControl|Sequence
    (:then_1
      (Variables|Parameters|SetIA_Bullet_Speed (Class|MovementComponent|GetMaxSpeed (Variables|Default|GetProjectileMovement))))))

(fn ConstructionScript)