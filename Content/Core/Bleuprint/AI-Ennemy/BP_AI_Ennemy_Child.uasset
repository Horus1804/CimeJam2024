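; Child enemy AI Blueprint that turns damage taken into score and combo for the player.
; After the parent's damage handling, it adds ScoreAdded to the player's score, multiplied by the current combo when above zero.
; It then resets the player's combo cooldown, increments the combo and pushes both values to the HUD.
; Any damage event triggers this while PlayerRef is valid; BeginPlay, Tick and construction just call the parent.
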(event EventBeginPlay
  (|CallParentFunction))

(event Collision|EventActorBeginOverlap
  (params (OtherActor :type Actor%20Object%20Reference)))

(event EventTick
  (params (DeltaSeconds :type Float%20%28single-precision%29))
  (|CallParentFunction DeltaSeconds))

(event Game|Damage|EventAnyDamage
  (params (Damage :type Float%20%28single-precision%29) (DamageType :type Damage%20Type%20Object%20Reference) (InstigatedBy :type Controller%20Object%20Reference) (DamageCauser :type Actor%20Object%20Reference))
  (bind _player_ref (Variables|Default|GetPlayer_Ref))
  (bind _player_ref_2 (Variables|Default|GetPlayer_Ref))
  (|CallParentFunction Damage DamageType InstigatedBy DamageCauser)
  (Utilities|FlowControl|Sequence
    (:then_0
      (bind _player_ref_3 (Variables|Default|GetPlayer_Ref)
        (:then
          (if (> (Variables|/Game/Core/Bleuprint/Player/BP_Player.BP_Player_C|GetCombo _player_ref_3) 0)
            (bind _output_get (Variables|/Game/Core/Bleuprint/Player/BP_Player.BP_Player_C|SetScore _player_ref_2 (+ (* (Variables|Default|GetScoreAdded) (Variables|/Game/Core/Bleuprint/Player/BP_Player.BP_Player_C|GetCombo _player_ref_3)) (Variables|/Game/Core/Bleuprint/Player/BP_Player.BP_Player_C|GetScore _player_ref_3))))
            (Default|SetScoreText (Variables|/Game/Core/Bleuprint/Player/BP_Player.BP_Player_C|GetHUD_Ref _player_ref_2) _output_get)
            (else
              (bind _output_get_2 (Variables|/Game/Core/Bleuprint/Player/BP_Player.BP_Player_C|SetScore _player_ref (+ (Variables|/Game/Core/Bleuprint/Player/BP_Player.BP_Player_C|GetScore _player_ref) (Variables|Default|GetScoreAdded))))
              (Default|SetScoreText (Variables|/Game/Core/Bleuprint/Player/BP_Player.BP_Player_C|GetHUD_Ref (Variables|Default|GetPlayer_Ref)) _output_get_2))))
        (:else)))
    (:then_1
      (bind _player_ref_4 (Variables|Default|GetPlayer_Ref)
        (:then
          (Variables|/Game/Core/Bleuprint/Player/BP_Player.BP_Player_C|SetCooldownCombo _player_ref_4 5)
          (bind _result (Math|Integer|IncrementInt (Variables|/Game/Core/Bleuprint/Player/BP_Player.BP_Player_C|GetCombo _player_ref_4))
            (:%20%20
              (Default|SetComboText (Variables|/Game/Core/Bleuprint/Player/BP_Player.BP_Player_C|GetHUD_Ref _player_ref_4) _result))))
        (:else)))))

(fn ConstructionScript
  (|CallParentFunction))