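; BP_AI_Ennemy is a forward-moving shooter enemy that picks a random Fire or Water element and one of six bullet patterns at spawn.
; A looping timer rolls a chance to fire spreads, player-aimed shots, sweeps or random sprays of BP_IA_Bullet, using nested timers for bursts.
; Each damage event removes one Health; death awards combo-multiplied score, raises the player's combo, updates the HUD and destroys the actor.
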(event Custom|Shoot_Event)

(event Custom|EventShoot4
  (bind _spawn_shoot_02 (Variables|Default|GetSpawn_Shoot_02))
  (bind _spawn_shoot_03 (Variables|Default|GetSpawn_Shoot_03))
  (bind _spawn_shoot_01 (Variables|Default|GetSpawn_Shoot_01))
  (bind _returnvalue (Transformation|GetWorldTransform _spawn_shoot_01))
  (bind _returnvalue_2 (Transformation|GetWorldTransform _spawn_shoot_02))
  (bind _returnvalue_3 (Transformation|GetWorldTransform _spawn_shoot_03))
  (bind _returnvalue_4 (Game|SpawnActorfromClass "/Game/Core/Bleuprint/AI-Ennemy/BP_IA_Bullet.BP_IA_Bullet_C" (Math|Transform|MakeTransform (.location _returnvalue) (.rotation _returnvalue) "1.000000,1.000000,1.000000") "Undefined" "MultiplyWithRoot" 0 0))
  (Utilities|IsValid _returnvalue_4
    (:Is%20Valid
      (Default|SetType _returnvalue_4 self)
      (bind _returnvalue_5 (Game|SpawnActorfromClass "/Game/Core/Bleuprint/AI-Ennemy/BP_IA_Bullet.BP_IA_Bullet_C" (Math|Transform|MakeTransform (.location _returnvalue_2) (.rotation _returnvalue_2) "1.000000,1.000000,1.000000") "Undefined" "MultiplyWithRoot" 0 0))
      (Utilities|IsValid _returnvalue_5
        (:Is%20Valid
          (Default|SetType _returnvalue_5 self)
          (bind _returnvalue_6 (Game|SpawnActorfromClass "/Game/Core/Bleuprint/AI-Ennemy/BP_IA_Bullet.BP_IA_Bullet_C" (Math|Transform|MakeTransform (.location _returnvalue_3) (.rotation _returnvalue_3) "1.000000,1.000000,1.000000") "Undefined" "MultiplyWithRoot" 0 0))
          (Utilities|IsValid _returnvalue_6
            (:Is%20Valid
              (Default|SetType _returnvalue_6 self))))))))

(event Custom|eventShoot6
  (bind _spawn_shoot_01 (Variables|Default|GetSpawn_Shoot_01))
  (bind _returnvalue (Transformation|GetWorldTransform _spawn_shoot_01))
  (if (!= (Variables|Default|GetNbr_Bullets) (Variables|Default|GetNbr_Max_Bullets))
    (Math|Integer|IncrementInt (Variables|Default|GetNbr_Bullets)
      (:%20%20
        (Transformation|SetRelativeRotation (Variables|Default|GetSpawn_Shoot_01) (Math|Rotator|MakeRotator 0.0 (Math|Random|RandomFloatinRange -6e+01 6e+01) -9e+01) false false)
        (bind _returnvalue_2 (Game|SpawnActorfromClass "/Game/Core/Bleuprint/AI-Ennemy/BP_IA_Bullet.BP_IA_Bullet_C" (Math|Transform|MakeTransform (.location _returnvalue) (.rotation _returnvalue) "1.000000,1.000000,1.000000") "Undefined" "MultiplyWithRoot" 0 0))
        (Utilities|IsValid _returnvalue_2
          (:Is%20Valid
            (Default|SetType _returnvalue_2 self)))))
    (else
      (Utilities|Time|ClearandInvalidateTimerbyHandle (Variables|Default|GetRefTimer%20Shoot)))))

(event Custom|eventShoot5
  (bind _spawn_shoot_01 (Variables|Default|GetSpawn_Shoot_01))
  (bind _spawn_shoot_01_2 (Variables|Default|GetSpawn_Shoot_01))
  (bind _returnvalue (Transformation|GetWorldTransform _spawn_shoot_01_2))
  (if (!= (Variables|Default|GetNbr_Bullets) (Variables|Default|GetNbr_Max_Bullets))
    (Math|Integer|IncrementInt (Variables|Default|GetNbr_Bullets)
      (:%20%20
        (bind _returnvalue_2 (Game|SpawnActorfromClass "/Game/Core/Bleuprint/AI-Ennemy/BP_IA_Bullet.BP_IA_Bullet_C" (Math|Transform|MakeTransform (.location _returnvalue) (.rotation _returnvalue) "1.000000,1.000000,1.000000") "Undefined" "MultiplyWithRoot" 0 0))
        (Utilities|IsValid _returnvalue_2
          (:Is%20Valid
            (Default|SetType _returnvalue_2 self)
            (Transformation|SetRelativeRotation _spawn_shoot_01 (Math|Rotator|MakeRotator 0.0 (+ (.pitch (Transformation|GetWorldRotation _spawn_shoot_01)) (Variables|Default|GetAngle_Rotation)) -9e+01) false false)))))
    (else
      (Utilities|Time|ClearandInvalidateTimerbyHandle (Variables|Default|GetRefTimer%20Shoot)))))

(event Custom|EventShoot2
  (bind _spawn_shoot_01 (Variables|Default|GetSpawn_Shoot_01))
  (bind _returnvalue (Transformation|GetWorldTransform _spawn_shoot_01))
  (if (!= (Variables|Default|GetNbr_Bullets) (Variables|Default|GetNbr_Max_Bullets))
    (Math|Integer|IncrementInt (Variables|Default|GetNbr_Bullets)
      (:%20%20
        (CallFunction|RotateShoottoPlayerFunction)
        (bind _returnvalue_2 (Game|SpawnActorfromClass "/Game/Core/Bleuprint/AI-Ennemy/BP_IA_Bullet.BP_IA_Bullet_C" (Math|Transform|MakeTransform (.location _returnvalue) (.rotation _returnvalue) "1.000000,1.000000,1.000000") "Undefined" "MultiplyWithRoot" 0 0))
        (Utilities|IsValid _returnvalue_2
          (:Is%20Valid
            (Default|SetType _returnvalue_2 self)))))
    (else
      (Utilities|Time|ClearandInvalidateTimerbyHandle (Variables|Default|GetRefTimer%20Shoot)))))

(event Custom|KillIA
  (bind _player_ref (Variables|BpRef|GetPlayer_Ref))
  (bind _player_ref_2 (Variables|BpRef|GetPlayer_Ref))
  (Utilities|FlowControl|Sequence
    (:then_0
      (bind _player_ref_3 (Variables|BpRef|GetPlayer_Ref)
        (:then
          (if (> (Variables|/Game/Core/Bleuprint/Player/BP_Player.BP_Player_C|GetCombo _player_ref_3) 0)
            (bind _output_get (Variables|/Game/Core/Bleuprint/Player/BP_Player.BP_Player_C|SetScore _player_ref_2 (+ (* (Variables|Default|GetScoreAdded) (Variables|/Game/Core/Bleuprint/Player/BP_Player.BP_Player_C|GetCombo _player_ref_3)) (Variables|/Game/Core/Bleuprint/Player/BP_Player.BP_Player_C|GetScore _player_ref_3))))
            (Default|SetScoreText (Variables|/Game/Core/Bleuprint/Player/BP_Player.BP_Player_C|GetHUD_Ref _player_ref_2) _output_get)
            (else
              (bind _output_get_2 (Variables|/Game/Core/Bleuprint/Player/BP_Player.BP_Player_C|SetScore _player_ref (+ (Variables|/Game/Core/Bleuprint/Player/BP_Player.BP_Player_C|GetScore _player_ref) (Variables|Default|GetScoreAdded))))
              (Default|SetScoreText (Variables|/Game/Core/Bleuprint/Player/BP_Player.BP_Player_C|GetHUD_Ref (Variables|BpRef|GetPlayer_Ref)) _output_get_2))))
        (:else)))
    (:then_1
      (bind _player_ref_4 (Variables|BpRef|GetPlayer_Ref)
        (:then
          (Variables|/Game/Core/Bleuprint/Player/BP_Player.BP_Player_C|SetCooldownCombo _player_ref_4 5)
          (bind _result (Math|Integer|IncrementInt (Variables|/Game/Core/Bleuprint/Player/BP_Player.BP_Player_C|GetCombo _player_ref_4))
            (:%20%20
              (Default|SetComboText (Variables|/Game/Core/Bleuprint/Player/BP_Player.BP_Player_C|GetHUD_Ref _player_ref_4) _result))))
        (:else)))
    (:then_2
      (Actor|DestroyActor))))

(event EventBeginPlay
  (Variables|/Script/Engine.FloatingPawnMovement|SetMaxSpeed (Variables|Default|GetFloatingPawnMovement) (Variables|Parameters|GetAI_Speed))
  (Utilities|FlowControl|Sequence
    (:then_0
      (bind _returnvalue (Actor|GetActorOfClass "/Game/Core/Bleuprint/AI-Ennemy/BP_IA_Bullet.BP_IA_Bullet_C"))
      (Variables|Bp_Ref|SetIA_Bullet_Ref _returnvalue)
      (bind _returnvalue_2 (Actor|GetActorOfClass "/Game/Core/Bleuprint/Player/BP_Player.BP_Player_C"))
      (Variables|BpRef|SetPlayer_Ref _returnvalue_2)
      (if (not (Utilities|Time|IsTimerActivebyHandle (Variables|Timer_Event_Ref|GetDebug_Print_Func_Ref)))
        (if (not (Utilities|Time|IsTimerActivebyHandle (Variables|TimerEventRef|GetIA_Shoot_Timer_Ref)))
          (CallFunction|SetIAElementsFunction)
          (Utilities|Time|SetTimerbyFunctionName 0 "Set_IA_Shoot_Paterns_Function" (Variables|Default|GetShootRate) true))))
    (:then_1
      (Variables|Boolean_Condition|SetCan_Shoot? false)
      (Variables|Parameters|SetAI_Speed (Class|MovementComponent|GetMaxSpeed (Variables|Default|GetFloatingPawnMovement)))
      (bind _output_get (Variables|Default|SetNbr_Max_Bullets 0))
      (Variables|Default|SetNbr_Bullets _output_get)
      (Variables|Enum|SetE_AI_Shoot_Patern (.OutItem (Utilities|Array|Random (Utilities|Array|MakeArray "NewEnumerator2" "NewEnumerator3" "NewEnumerator4" "NewEnumerator5" "NewEnumerator6" "NewEnumerator7")))))))

(event Game|Damage|EventAnyDamage
  (params (Damage :type Float%20%28single-precision%29) (DamageType :type Damage%20Type%20Object%20Reference) (InstigatedBy :type Controller%20Object%20Reference) (DamageCauser :type Actor%20Object%20Reference))
  (bind _result (Math|Integer|DecrementInt (Variables|Default|GetHealth))
    (:%20%20
      (if (== _result 0)
        (CallFunction|KillIA)))))

(event EventTick
  (params (DeltaSeconds :type Float%20%28single-precision%29))
  (Utilities|FlowControl|Sequence
    (:then_1
      (CallFunction|MoveForwardFunction))))

(fn ConstructionScript)

(fn DebugPrintFunction)

(fn MoveForwardFunction
  (Pawn|Input|AddMovementInput (* (Math|Vector|GetForwardVector (Transformation|GetActorRotation)) (Variables|Parameters|GetAI_Speed)) 1.0 false))

(fn SetIAElementsFunction
  (bind _skeletalmesh (Variables|Default|GetSkeletalMesh))
  (bind _output_get (Variables|Enum|SetE_AI_Elements (.OutItem (Utilities|Array|Random (Utilities|Array|MakeArray "NewEnumerator0" "NewEnumerator1")))))
  (switch Utilities|FlowControl|Switch|SwitchonE_IA_Ennemy_Elements _output_get
    (:NewEnumerator0
      (Rendering|Material|SetMaterial _skeletalmesh 1 0)
      (Development|PrintString "IA_Fire" true true "(R=0.117647,G=1.000000,B=0.000000,A=1.000000)"))
    (:NewEnumerator1
      (Rendering|Material|SetMaterial _skeletalmesh 1 "/Game/Core/VFX/Luos8Elements/Materials/Aqua/M_LMagic_Water_01.M_LMagic_Water_01")
      (Development|PrintString "IA_Water" true true "(R=0.117647,G=1.000000,B=0.000000,A=1.000000)"))))

(fn SetIAShootPaternsFunction
  (bind _spawn_shoot_04 (Variables|Default|GetSpawn_Shoot_04))
  (bind _spawn_shoot_01 (Variables|Default|GetSpawn_Shoot_01))
  (bind _spawn_shoot_06 (Variables|Default|GetSpawn_Shoot_06))
  (bind _spawn_shoot_01_2 (Variables|Default|GetSpawn_Shoot_01))
  (bind _spawn_shoot_02 (Variables|Default|GetSpawn_Shoot_02))
  (bind _spawn_shoot_03 (Variables|Default|GetSpawn_Shoot_03))
  (bind _spawn_shoot_01_3 (Variables|Default|GetSpawn_Shoot_01))
  (bind _spawn_shoot_01_4 (Variables|Default|GetSpawn_Shoot_01))
  (bind _spawn_shoot_05 (Variables|Default|GetSpawn_Shoot_05))
  (bind _spawn_shoot_01_5 (Variables|Default|GetSpawn_Shoot_01))
  (bind _spawn_shoot_07 (Variables|Default|GetSpawn_Shoot_07))
  (bind _returnvalue (Transformation|GetWorldTransform _spawn_shoot_04))
  (bind _returnvalue_2 (Transformation|GetWorldTransform _spawn_shoot_07))
  (bind _returnvalue_3 (Transformation|GetWorldTransform _spawn_shoot_01))
  (bind _returnvalue_4 (Transformation|GetWorldTransform _spawn_shoot_06))
  (bind _returnvalue_5 (Transformation|GetWorldTransform _spawn_shoot_01_2))
  (bind _returnvalue_6 (Transformation|GetWorldTransform _spawn_shoot_02))
  (bind _returnvalue_7 (Transformation|GetWorldTransform _spawn_shoot_03))
  (bind _returnvalue_8 (Transformation|GetWorldTransform _spawn_shoot_01_3))
  (bind _returnvalue_9 (Transformation|GetWorldTransform _spawn_shoot_05))
  (bind _returnvalue_10 (Transformation|GetWorldTransform _spawn_shoot_01_4))
  (if (> (Math|Random|RandomIntegerinRange 0 100) (Variables|Default|GetProbashoot))
    (switch Utilities|FlowControl|Switch|SwitchonE_IA_Shoot_Paterns (Variables|Enum|GetE_AI_Shoot_Patern)
      (:NewEnumerator2
        (bind _returnvalue_11 (Game|SpawnActorfromClass "/Game/Core/Bleuprint/AI-Ennemy/BP_IA_Bullet.BP_IA_Bullet_C" (Math|Transform|MakeTransform (.location _returnvalue_8) (.rotation _returnvalue_8) "1.000000,1.000000,1.000000") "Undefined" "MultiplyWithRoot" 0 0))
        (Utilities|IsValid _returnvalue_11
          (:Is%20Valid
            (Default|SetType _returnvalue_11 self)
            (bind _returnvalue_12 (Game|SpawnActorfromClass "/Game/Core/Bleuprint/AI-Ennemy/BP_IA_Bullet.BP_IA_Bullet_C" (Math|Transform|MakeTransform (.location _returnvalue_6) (.rotation _returnvalue_6) "1.000000,1.000000,1.000000") "Undefined" "MultiplyWithRoot" 0 0))
            (Utilities|IsValid _returnvalue_12
              (:Is%20Valid
                (Default|SetType _returnvalue_12 self)
                (bind _returnvalue_13 (Game|SpawnActorfromClass "/Game/Core/Bleuprint/AI-Ennemy/BP_IA_Bullet.BP_IA_Bullet_C" (Math|Transform|MakeTransform (.location _returnvalue_7) (.rotation _returnvalue_7) "1.000000,1.000000,1.000000") "Undefined" "MultiplyWithRoot" 0 0))
                (Utilities|IsValid _returnvalue_13
                  (:Is%20Valid
                    (Default|SetType _returnvalue_13 self)
                    (bind _returnvalue_14 (Game|SpawnActorfromClass "/Game/Core/Bleuprint/AI-Ennemy/BP_IA_Bullet.BP_IA_Bullet_C" (Math|Transform|MakeTransform (.location _returnvalue) (.rotation _returnvalue) "1.000000,1.000000,1.000000") "Undefined" "MultiplyWithRoot" 0 0))
                    (Utilities|IsValid _returnvalue_14
                      (:Is%20Valid
                        (Default|SetType _returnvalue_14 self)
                        (bind _returnvalue_15 (Game|SpawnActorfromClass "/Game/Core/Bleuprint/AI-Ennemy/BP_IA_Bullet.BP_IA_Bullet_C" (Math|Transform|MakeTransform (.location _returnvalue_9) (.rotation _returnvalue_9) "1.000000,1.000000,1.000000") "Undefined" "MultiplyWithRoot" 0 0))
                        (Utilities|IsValid _returnvalue_15
                          (:Is%20Valid
                            (Default|SetType _returnvalue_15 self))))))))))))
      (:NewEnumerator3
        (Variables|Default|SetNbr_Max_Bullets (Math|Random|RandomIntegerinRange 3 5))
        (Variables|Default|SetNbr_Bullets 0)
        (bind _returnvalue_16 (Utilities|Time|SetTimerbyEvent (EventDispatchers|CreateEvent :!event Custom|EventShoot2) 0.1 true))
        (Variables|Default|SetRefTimer%20Shoot _returnvalue_16))
      (:NewEnumerator4
        (bind _returnvalue_17 (Game|SpawnActorfromClass "/Game/Core/Bleuprint/AI-Ennemy/BP_IA_Bullet.BP_IA_Bullet_C" (Math|Transform|MakeTransform (+ (.location _returnvalue_3) "-50.000000,0.000000,0.000000") (.rotation _returnvalue_3) "1.000000,1.000000,1.000000") "Undefined" "MultiplyWithRoot" 0 0))
        (Utilities|IsValid _returnvalue_17
          (:Is%20Valid
            (Default|SetType _returnvalue_17 self)
            (bind _returnvalue_18 (Game|SpawnActorfromClass "/Game/Core/Bleuprint/AI-Ennemy/BP_IA_Bullet.BP_IA_Bullet_C" (Math|Transform|MakeTransform (.location _returnvalue_4) (.rotation _returnvalue_4) "1.000000,1.000000,1.000000") "Undefined" "MultiplyWithRoot" 0 0))
            (Utilities|IsValid _returnvalue_18
              (:Is%20Valid
                (Default|SetType _returnvalue_18 self)
                (bind _returnvalue_19 (Game|SpawnActorfromClass "/Game/Core/Bleuprint/AI-Ennemy/BP_IA_Bullet.BP_IA_Bullet_C" (Math|Transform|MakeTransform (.location _returnvalue_2) (.rotation _returnvalue_2) "1.000000,1.000000,1.000000") "Undefined" "MultiplyWithRoot" 0 0))
                (Utilities|IsValid _returnvalue_19
                  (:Is%20Valid
                    (Default|SetType _returnvalue_19 self))))))))
      (:NewEnumerator5
        (CallFunction|RotateShoottoPlayerFunction)
        (CallFunction|EventShoot4)
        (Utilities|Time|SetTimerbyEvent (EventDispatchers|CreateEvent :!event Custom|EventShoot4) 0.2))
      (:NewEnumerator6
        (bind _output_get (Variables|Default|SetAngle_Rotation (Math|Float|SelectFloat -17.142857 17.142857 (Math|Random|RandomBool))))
        (if (< _output_get 0.0)
          (Transformation|SetRelativeRotation (Variables|Default|GetSpawn_Shoot_01) (Math|Rotator|MakeRotator 0.0 6e+01 -9e+01) false false)
          (else
            (Transformation|SetRelativeRotation (Variables|Default|GetSpawn_Shoot_01) (Math|Rotator|MakeRotator 0.0 -6e+01 -9e+01) false false)))
        (bind _returnvalue_20 (Game|SpawnActorfromClass "/Game/Core/Bleuprint/AI-Ennemy/BP_IA_Bullet.BP_IA_Bullet_C" (Math|Transform|MakeTransform (.location _returnvalue_10) (.rotation _returnvalue_10) "1.000000,1.000000,1.000000") "Undefined" "MultiplyWithRoot" 0 0))
        (Utilities|IsValid _returnvalue_20
          (:Is%20Valid
            (Default|SetType _returnvalue_20 self)
            (Transformation|SetRelativeRotation _spawn_shoot_01_5 (Math|Rotator|MakeRotator 0.0 (+ (.pitch (Transformation|GetWorldRotation _spawn_shoot_01_5)) (Variables|Default|GetAngle_Rotation)) -9e+01) false false)
            (Variables|Default|SetNbr_Bullets 0)
            (Variables|Default|SetNbr_Max_Bullets 7)
            (bind _returnvalue_21 (Utilities|Time|SetTimerbyEvent (EventDispatchers|CreateEvent :!event Custom|eventShoot5) 0.1 true))
            (Variables|Default|SetRefTimer%20Shoot _returnvalue_21))))
      (:NewEnumerator7
        (Transformation|SetRelativeRotation (Variables|Default|GetSpawn_Shoot_01) (Math|Rotator|MakeRotator 0.0 (Math|Random|RandomFloatinRange -6e+01 6e+01) -9e+01) false false)
        (bind _returnvalue_22 (Game|SpawnActorfromClass "/Game/Core/Bleuprint/AI-Ennemy/BP_IA_Bullet.BP_IA_Bullet_C" (Math|Transform|MakeTransform (.location _returnvalue_5) (.rotation _returnvalue_5) "1.000000,1.000000,1.000000") "Undefined" "MultiplyWithRoot" 0 0))
        (Utilities|IsValid _returnvalue_22
          (:Is%20Valid
            (Default|SetType _returnvalue_22 self)
            (Variables|Default|SetNbr_Max_Bullets 5)
            (Variables|Default|SetNbr_Bullets 0)
            (bind _returnvalue_23 (Utilities|Time|SetTimerbyEvent (EventDispatchers|CreateEvent :!event Custom|eventShoot6) 0.1 true))
            (Variables|Default|SetRefTimer%20Shoot _returnvalue_23)))))))

(fn RotateShoottoPlayerFunction
  (Transformation|SetRelativeRotation (Variables|Default|GetSpawn_Shoot_01) (Math|Rotator|MakeRotator 0.0 (Math|Float|Clamp(Float) (.Pitch (Math|Rotator|BreakRotator (Math|Rotator|FindLookatRotation (Transformation|GetWorldLocation (Variables|Default|GetSpawn_Shoot_01)) (Transformation|GetActorLocation (Variables|BpRef|GetPlayer_Ref))))) -8e+01 8e+01) -9e+01) false false))