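; Enemy spawner actor that releases escalating waves of BP_AI_Ennemy ahead of the camera.
; A looping cooldown timer starts at BeginPlay, and SpawnSystem spawns each batch at a fixed X offset from the camera with random height, passing each enemy the player reference.
; A wave counter raises the batch size whenever it hits a multiple of a threshold, then resets and doubles that threshold, so increases come progressively less often.
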(event Custom|SpawnEnnemies
  (bind _returnvalue (Game|SpawnActorfromClass "/Game/Core/Bleuprint/AI-Ennemy/BP_AI_Ennemy.BP_AI_Ennemy_C" (Math|Transform|MakeTransform (Math|Vector|MakeVector (+ (.x (Transformation|GetActorLocation (Variables|Default|GetCameraRef))) 3e+03) 0.0 (Math|Random|RandomFloatinRange -1.1e+03 1.8e+03)) "0.000000,-180.000000,0.000000" "1.000000,1.000000,1.000000") "Undefined" "MultiplyWithRoot" 0 0))
  (Utilities|IsValid _returnvalue
    (:Is%20Valid
      (Variables|/Game/Core/Bleuprint/AI-Ennemy/BP_AI_Ennemy.BP_AI_Ennemy_C|SetPlayer_Ref _returnvalue (Variables|Default|GetPlayerRef)))))

(event Custom|Next%20wave
  (Development|PrintString (Utilities|String|Append (Utilities|String|ToString(Integer) (Variables|Default|GetSpawnAmount)) " | " (Utilities|String|ToString(Integer) (Variables|Default|GetSpawnnextAmount))))
  (if (== (Math|Integer|%(Integer) (Variables|Default|GetSpawnAmount) (Variables|Default|GetSpawnnextAmount)) 0)
    (Variables|Default|SetSpawnnextAmount (* (Variables|Default|GetSpawnnextAmount) 2))
    (Development|PrintString "plus d enemy")
    (Variables|Default|SetSpawnAmount 0)
    (Math|Integer|IncrementInt (Variables|Default|GetspawnEnemyAmound))))

(event Custom|SpawnSystem
  (for _index (range 0 (- (Variables|Default|GetspawnEnemyAmound) 1))
    (CallFunction|SpawnEnnemies))
  (CallFunction|NextWave)
  (Math|Integer|IncrementInt (Variables|Default|GetSpawnAmount)))

(event EventBeginPlay
  (Utilities|Time|SetTimerbyEvent (EventDispatchers|CreateEvent :!event Custom|SpawnSystem) (Variables|Default|GetSpawnCooldown) true)
  (Variables|Default|SetSpawnnextAmount 2))

(fn ConstructionScript)