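; Player pawn driven by Enhanced Input, with planar movement and an unfinished shooting action.
; On BeginPlay it adds the input mapping context to BP_CustomPlayerController and switches the view to RefCamera.
; Move input feeds FloatingPawnMovement along world Z and X, with a debug "Hello" print.
; Shot input starts a looping timer on ShopEvent, which is still empty, with an unconnected SpawnActor node left in the graph.
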(event Custom|ShopEvent)

(event Input|EnhancedActionEvents|EnhancedInputActionAi_Move
  (params (ActionValue :type Vector%202D%20Structure) (ElapsedSeconds :type Float%20%28double-precision%29) (TriggeredSeconds :type Float%20%28double-precision%29) (InputAction :type Input%20Action%20Object%20Reference :default "/Game/Core/Bleuprint/Input/Action/Ai_Move.Ai_Move"))
  (Development|PrintString "Hello")
  (Class|PawnMovementComponent|AddInputVector (Variables|Default|GetFloatingPawnMovement) (Math|Vector|MakeVector 0.0 0.0 (.x ActionValue)) false)
  (Class|PawnMovementComponent|AddInputVector (Variables|Default|GetFloatingPawnMovement) (Math|Vector|MakeVector (.y ActionValue) 0.0 0.0) false))

(event Input|EnhancedActionEvents|EnhancedInputActionAI_Shot
  (params (ActionValue :type Boolean) (ElapsedSeconds :type Float%20%28double-precision%29) (TriggeredSeconds :type Float%20%28double-precision%29) (InputAction :type Input%20Action%20Object%20Reference :default "/Game/Core/Bleuprint/Input/Action/AI_Shot.AI_Shot"))
  (:Started
    (Utilities|Time|SetTimerbyEvent (delegate Custom|ShopEvent) 0.5 true)))

(event EventBeginPlay
  (bind _asbp_custom_player_controller (Utilities|Casting|CastToBP_CustomPlayerController (Pawn|GetController)))
  (Input|AddMappingContext (PlayerController|LocalPlayerSubsystems|GetEnhancedInputLocalPlayerSubsystem _asbp_custom_player_controller) "/Game/Core/Bleuprint/Input/IMC_Input.IMC_Input" 0 "(bIgnoreAllPressedKeysUntilRelease=True,bForceImmediately=False,bNotifyUserSettings=False)")
  (Game|Player|SetViewTargetwithBlend _asbp_custom_player_controller (Variables|Default|GetRefCamera) 0.0 "VTBlend_Linear" 0.0 false))

(event Collision|EventActorBeginOverlap
  (params (OtherActor :type Actor%20Object%20Reference)))

(event EventTick
  (params (DeltaSeconds :type Float%20%28single-precision%29)))

(fn ConstructionScript)