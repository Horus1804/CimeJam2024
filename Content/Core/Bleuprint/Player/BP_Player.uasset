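; Player pawn for a side-scrolling shooter, scrolling along X each tick until KillTickForBoss is set, viewed through RefCamera.
; Enhanced Input drives X/Z movement, pausing, and timer-repeated fire of three-arrow projectile spreads and rocks spawned below.
; A FlipFlop swaps the fire/water shield, and enemy bullets only cost health when their element differs, ending in Game Over.
; The HUD shows health, element and a combo that resets when its cooldown expires.
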(event Custom|DecreaseCooldownCombo
  (bind _hud_ref (Variables|Default|GetHUD_Ref))
  (if (!= (Variables|Default|GetCooldownCombo) 0)
    (Math|Integer|DecrementInt (Variables|Default|GetCooldownCombo))
    (else
      (bind _output_get (Variables|Default|SetCombo 0))
      (Default|SetComboText _hud_ref _output_get)
      (Widget|SetVisibility (Variables|/Game/Core/Bleuprint/UI/WBP_HUD.WBP_HUD_C|GetText_Combo _hud_ref) "Hidden"))))

(event Custom|ShotRocheEvent
  (bind _returnvalue (Transformation|GetActorTransform))
  (Game|SpawnActorfromClass "/Game/Core/Bleuprint/Player/Projo/BP_ProjoRoch.BP_ProjoRoch_C" (Math|Transform|MakeTransform (+ (.location _returnvalue) "0.000000,0.000000,-120.000000") (.rotation _returnvalue) (.scale _returnvalue)) "Undefined" "MultiplyWithRoot" 0 0)
  (Variables|Default|SetIsShotRock true))

(event Custom|ResetShot
  (Variables|Default|SetIsShot true))

(event Custom|ResetShotRock
  (Variables|Default|SetIsShotRock true))

(event Custom|Debug%20damage
  (bind _result (Math|Integer|DecrementInt (Variables|Default|GetHealth))
    (:%20%20
      (Default|SetHealthBar (Variables|Default|GetHUD_Ref) _result)
      (if (== _result 0)
        (Development|PrintString "You are Dead" true true "(R=0.000000,G=0.000000,B=0.000000,A=1.000000)" 2e+01)
        (bind _returnvalue (UserInterface|CreateWidget "/Game/Core/Bleuprint/UI/WBP_GameOver.WBP_GameOver_C"))
        (UserInterface|Viewport|AddtoViewport _returnvalue 0)))))

(event Custom|ShotEvent
  (Game|SpawnActorfromClass "/Game/Core/Bleuprint/Player/Projo/BP_ProjoPlayer.BP_ProjoPlayer_C" (Transformation|GetWorldTransform (Variables|Default|GetArrow)) "Undefined" "MultiplyWithRoot" 0 0)
  (Game|SpawnActorfromClass "/Game/Core/Bleuprint/Player/Projo/BP_ProjoPlayer.BP_ProjoPlayer_C" (Transformation|GetWorldTransform (Variables|Default|GetArrow1)) "Undefined" "MultiplyWithRoot" 0 0)
  (Game|SpawnActorfromClass "/Game/Core/Bleuprint/Player/Projo/BP_ProjoPlayer.BP_ProjoPlayer_C" (Transformation|GetWorldTransform (Variables|Default|GetArrow2)) "Undefined" "MultiplyWithRoot" 0 0)
  (Variables|Default|SetIsShot true))

(event Input|EnhancedActionEvents|EnhancedInputActionAi_Move
  (params (ActionValue :type Vector%202D%20Structure) (ElapsedSeconds :type Float%20%28double-precision%29) (TriggeredSeconds :type Float%20%28double-precision%29) (InputAction :type Input%20Action%20Object%20Reference :default "/Game/Core/Bleuprint/Player/Input/Action/Ai_Move.Ai_Move"))
  (Pawn|Input|AddMovementInput "0.000000,0.000000,1.000000" (.x ActionValue) false)
  (Pawn|Input|AddMovementInput "1.000000,0.000000,0.000000" (.y ActionValue) false))

(event Input|EnhancedActionEvents|EnhancedInputActionAI_Shot
  (params (ActionValue :type Boolean) (ElapsedSeconds :type Float%20%28double-precision%29) (TriggeredSeconds :type Float%20%28double-precision%29) (InputAction :type Input%20Action%20Object%20Reference :default "/Game/Core/Bleuprint/Player/Input/Action/AI_Shot.AI_Shot"))
  (:Started
    (if (Variables|Default|GetIsShot)
      (Variables|Default|SetIsShot false)
      (bind _returnvalue (Utilities|Time|SetTimerbyEvent (EventDispatchers|CreateEvent :!event Custom|ShotEvent) (Variables|Default|GetTimerShot) true))
      (Variables|Default|SetRefTimerShot _returnvalue)
      (Utilities|Time|SetTimerbyEvent (delegate Custom|ResetShot) (Variables|Default|GetTimerShot))
      (Game|SpawnActorfromClass "/Game/Core/Bleuprint/Player/Projo/BP_ProjoPlayer.BP_ProjoPlayer_C" (Transformation|GetWorldTransform (Variables|Default|GetArrow)) "Undefined" "MultiplyWithRoot" 0 0)
      (Game|SpawnActorfromClass "/Game/Core/Bleuprint/Player/Projo/BP_ProjoPlayer.BP_ProjoPlayer_C" (Transformation|GetWorldTransform (Variables|Default|GetArrow1)) "Undefined" "MultiplyWithRoot" 0 0)
      (Game|SpawnActorfromClass "/Game/Core/Bleuprint/Player/Projo/BP_ProjoPlayer.BP_ProjoPlayer_C" (Transformation|GetWorldTransform (Variables|Default|GetArrow2)) "Undefined" "MultiplyWithRoot" 0 0)))
  (:Completed
    (Utilities|Time|ClearandInvalidateTimerbyHandle (Variables|Default|GetRefTimerShot))))

(event Input|EnhancedActionEvents|EnhancedInputActionAI_Roche
  (params (ActionValue :type Boolean) (ElapsedSeconds :type Float%20%28double-precision%29) (TriggeredSeconds :type Float%20%28double-precision%29) (InputAction :type Input%20Action%20Object%20Reference :default "/Game/Core/Bleuprint/Player/Input/Action/AI_Roche.AI_Roche"))
  (bind _returnvalue (Transformation|GetActorTransform))
  (:Started
    (if (Variables|Default|GetIsShotRock)
      (Variables|Default|SetIsShotRock false)
      (bind _returnvalue_2 (Utilities|Time|SetTimerbyEvent (EventDispatchers|CreateEvent :!event Custom|ShotRocheEvent) (Variables|Default|GetTimerShotRock) true))
      (Variables|Default|SetRefTimerRock _returnvalue_2)
      (Utilities|Time|SetTimerbyEvent (delegate Custom|ResetShotRock) (Variables|Default|GetTimerShotRock))
      (Game|SpawnActorfromClass "/Game/Core/Bleuprint/Player/Projo/BP_ProjoRoch.BP_ProjoRoch_C" (Math|Transform|MakeTransform (+ (.location _returnvalue) "0.000000,0.000000,-100.000000") (.rotation _returnvalue) (.scale _returnvalue)) "Undefined" "MultiplyWithRoot" 0 0)))
  (:Completed
    (Utilities|Time|ClearandInvalidateTimerbyHandle (Variables|Default|GetRefTimerRock))))

(event Input|EnhancedActionEvents|EnhancedInputActionAI_SwapShield
  (params (ActionValue :type Boolean) (ElapsedSeconds :type Float%20%28double-precision%29) (TriggeredSeconds :type Float%20%28double-precision%29) (InputAction :type Input%20Action%20Object%20Reference :default "/Game/Core/Bleuprint/Player/Input/Action/AI_SwapShield.AI_SwapShield"))
  (:Started
    (Utilities|FlowControl|FlipFlop
      (:A
        (Rendering|Material|SetMaterial (Variables|Default|GetSphere) 0 "/Game/Core/Material/Inst/M_Shield_Water_Inst.M_Shield_Water_Inst")
        (Variables|Default|SetETypeShield "NewEnumerator1")
        (Default|SetElementIcon (Variables|Default|GetHUD_Ref) "/Game/Core/Bleuprint/UI/Images/ElementsIcons/icon_water.icon_water"))
      (:B
        (Rendering|Material|SetMaterial (Variables|Default|GetSphere) 0 "/Game/Core/Material/Inst/M_Shield_Fire_Inst.M_Shield_Fire_Inst")
        (Variables|Default|SetETypeShield "NewEnumerator0")
        (Default|SetElementIcon (Variables|Default|GetHUD_Ref) "/Game/Core/Bleuprint/UI/Images/ElementsIcons/icon_fire.icon_fire")))))

(event Input|EnhancedActionEvents|EnhancedInputActionIA_Pause
  (params (ActionValue :type Boolean) (ElapsedSeconds :type Float%20%28double-precision%29) (TriggeredSeconds :type Float%20%28double-precision%29) (InputAction :type Input%20Action%20Object%20Reference :default "/Game/Core/Bleuprint/Player/Input/Action/IA_Pause.IA_Pause"))
  (bind _returnvalue (UserInterface|CreateWidget "/Game/Core/Bleuprint/UI/WBP_Pause.WBP_Pause_C"))
  (UserInterface|Viewport|AddtoViewport _returnvalue 0))

(event EventBeginPlay
  (bind _asbp_custom_player_controller (Utilities|Casting|CastToBP_CustomPlayerController (Pawn|GetController)))
  (Input|AddMappingContext (PlayerController|LocalPlayerSubsystems|GetEnhancedInputLocalPlayerSubsystem _asbp_custom_player_controller) "/Game/Core/Bleuprint/Player/Input/IMC_Input.IMC_Input" 0 "(bIgnoreAllPressedKeysUntilRelease=True,bForceImmediately=False,bNotifyUserSettings=False)")
  (Game|Player|SetViewTargetwithBlend _asbp_custom_player_controller (Variables|Default|GetRefCamera) 0.0 "VTBlend_Linear" 0.0 false)
  (Variables|/Script/Engine.FloatingPawnMovement|SetMaxSpeed (Variables|Default|GetFloatingPawnMovement) (Variables|Default|GetMax%20Speed))
  (Utilities|Time|SetTimerbyEvent (EventDispatchers|CreateEvent :!event Custom|DecreaseCooldownCombo) 1.0 true)
  (bind _returnvalue (UserInterface|CreateWidget "/Game/Core/Bleuprint/UI/WBP_HUD.WBP_HUD_C"))
  (bind _output_get (Variables|Default|SetHUD_Ref _returnvalue))
  (UserInterface|Viewport|AddtoViewport _output_get 0)
  (Variables|Default|SetUsername (Variables|/Game/Core/Bleuprint/SaveSystem/BP_CustomSaveGame.BP_CustomSaveGame_C|GetUsername (Variables|/Game/Core/Bleuprint/SaveSystem/BP_CustomGameInstance.BP_CustomGameInstance_C|GetSaveGameRef (.AsBP%20Custom%20Game%20Instance (Utilities|Casting|CastToBP_CustomGameInstance (Game|GetGameInstance)))))))

(event Collision|EventActorBeginOverlap
  (params (OtherActor :type Actor%20Object%20Reference)))

(event EventTick
  (params (DeltaSeconds :type Float%20%28single-precision%29))
  (bind _hud_ref (Variables|Default|GetHUD_Ref))
  (Utilities|FlowControl|Sequence
    (:then_0
      (if (> (Variables|Default|GetCombo) 0)
        (Widget|SetVisibility (Variables|/Game/Core/Bleuprint/UI/WBP_HUD.WBP_HUD_C|GetText_Combo _hud_ref) "Visible")
        (Default|SetComboText _hud_ref (Variables|Default|GetCombo))))
    (:then_1
      (if (not (Variables|Default|GetKill_Tick_For_Boss))
        (Transformation|SetActorLocation (+ (Transformation|GetActorLocation) "10.000000,0.000000,0.000000") false false)))))

(event Game|Damage|EventAnyDamage
  (params (Damage :type Float%20%28single-precision%29) (DamageType :type Damage%20Type%20Object%20Reference) (InstigatedBy :type Controller%20Object%20Reference) (DamageCauser :type Actor%20Object%20Reference))
  (Utilities|FlowControl|Sequence
    (:then_0
      (bind _asbp_ia_bullet (Utilities|Casting|CastToBP_IA_Bullet DamageCauser))
      (bind _ia_ennemy_ref (Variables|/Game/Core/Bleuprint/AI-Ennemy/BP_IA_Bullet.BP_IA_Bullet_C|GetIA_Ennemy_Ref _asbp_ia_bullet)
        (:then
          (if (Utilities|Enum|NotEqual(Enum) (Variables|/Game/Core/Bleuprint/AI-Ennemy/BP_AI_Ennemy.BP_AI_Ennemy_C|GetE_AI_Elements _ia_ennemy_ref) (Variables|Default|GetETypeShield))
            (bind _result (Math|Integer|DecrementInt (Variables|Default|GetHealth) :!label _label)
              (:%20%20
                (Default|SetHealthBar (Variables|Default|GetHUD_Ref) _result)
                (if (== _result 0)
                  (Development|PrintString "You are Dead" true true "(R=0.000000,G=0.000000,B=0.000000,A=1.000000)" 2e+01)
                  (bind _returnvalue (UserInterface|CreateWidget "/Game/Core/Bleuprint/UI/WBP_GameOver.WBP_GameOver_C"))
                  (UserInterface|Viewport|AddtoViewport _returnvalue 0))))))
        (:else)))
    (:then_1
      (bind _asbp_test_bullet (Utilities|Casting|CastToBP_TestBullet DamageCauser))
      (if (Utilities|Enum|NotEqual(Enum) (Variables|/Game/Core/GD_Test/BP_TestBullet.BP_TestBullet_C|GetE_IA_Elements _asbp_test_bullet) (Variables|Default|GetETypeShield))
        (goto _label)))))

(fn ConstructionScript
  (Transformation|SetRelativeRotation (Variables|Default|GetArrow1) (Math|Rotator|MakeRotator 0.0 (Variables|Default|GetNew%20Rotation%20Haut) 0.0) false false)
  (Transformation|SetRelativeRotation (Variables|Default|GetArrow2) (Math|Rotator|MakeRotator 0.0 (Variables|Default|GetNew%20Rotation%20Bas) 0.0) false false))